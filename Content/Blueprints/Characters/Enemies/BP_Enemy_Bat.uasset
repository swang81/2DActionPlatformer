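; BP_Enemy_Bat is a bat enemy that patrols endlessly back and forth between two points.
; On BeginPlay it caches the world locations of its TopPos and BottonPos components and sets the MoveAnim timeline's play rate from MovePlayRate.
; The timeline lerps the actor between those points without sweeping, and a FlipFlop on Finished alternates reverse and forward playback.
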(event Custom|MoveForward
  (bind _alpha (Timeline|MoveAnim PlayFromStart)
    (:Update
      (Transformation|SetActorLocation (Math|Vector|Lerp(Vector) (Variables|Default|GetWorldTopPos) (Variables|Default|GetWorldBottomPos) _alpha) false false))
    (:Finished
      (Utilities|FlowControl|FlipFlop
        (:A
          (CallFunction|MoveBackForward))
        (:B
          (CallFunction|MoveForward))))))

(event Custom|MoveBackForward
  (bind _alpha (Timeline|MoveAnim ReverseFromEnd)
    (:Update
      (Transformation|SetActorLocation (Math|Vector|Lerp(Vector) (Variables|Default|GetWorldTopPos) (Variables|Default|GetWorldBottomPos) _alpha) false false))
    (:Finished
      (Utilities|FlowControl|FlipFlop
        (:A
          (CallFunction|MoveBackForward))
        (:B
          (CallFunction|MoveForward))))))

(event EventBeginPlay
  (|CallParentFunction)
  (Variables|Default|SetWorldTopPos (Transformation|GetWorldLocation (Variables|Default|GetTopPos)))
  (Variables|Default|SetWorldBottomPos (Transformation|GetWorldLocation (Variables|Default|GetBottonPos)))
  (Components|Timeline|SetPlayRate (Variables|Default|GetMoveAnim) (Variables|Default|GetMovePlayRate))
  (CallFunction|MoveForward))

(event Collision|EventActorBeginOverlap
  (params (OtherActor :type Actor%20Object%20Reference))
  (|CallParentFunction OtherActor) ; This node is disabled and will not be called.\nDrag off pins to build functionality.
)

(event EventTick
  (params (DeltaSeconds :type Float%20%28single-precision%29))
  (|CallParentFunction DeltaSeconds) ; This node is disabled and will not be called.\nDrag off pins to build functionality.
)

(fn ConstructionScript
  (|CallParentFunction))