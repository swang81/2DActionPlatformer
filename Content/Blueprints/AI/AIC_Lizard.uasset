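; AI controller for the lizard enemy that makes it shoot fireballs at a regular interval.
; On possess it casts the pawn to BP_Enemy_Lizard, stores it and starts a looping timer using the shoot interval.
; A custom event tells the stored lizard to shoot a fireball, with no targeting or movement logic in the controller.
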(event Custom|ShootProjetile
  (Default|ShootFireball (Variables|Default|GetOwningLizard)))

(event EventBeginPlay
  (|CallParentFunction) ; This node is disabled and will not be called.\nDrag off pins to build functionality.
)

(event EventTick
  (params (DeltaSeconds :type Float%20%28single-precision%29))
  (|CallParentFunction DeltaSeconds) ; This node is disabled and will not be called.\nDrag off pins to build functionality.
)

(event EventPossess
  (params (PossessedPawn :type Pawn%20Object%20Reference))
  (bind _asbp_enemy_lizard (Utilities|Casting|CastToBP_Enemy_Lizard PossessedPawn))
  (Variables|Default|SetOwningLizard _asbp_enemy_lizard)
  (Utilities|Time|SetTimerbyEvent (EventDispatchers|CreateEvent :!event Custom|ShootProjetile) (Variables|Default|GetShootInterval) true))

(fn ConstructionScript
  (|CallParentFunction))